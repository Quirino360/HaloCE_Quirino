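; Enemy Blueprint for an AI character that carries a gun and shoots when commanded.
; It repositions its FPGun on begin play and exposes start and stop shooting events that toggle the weapon's CanShoot flag.
; AI Perception updates write the sensed state of the player into the PlayerOnSight blackboard key.
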(event `self.ReceiveBeginPlay`
  (`SceneComponent.K2_SetRelativeLocationAndRotation` (`self.FP_Gun`) (40.0 30.0 40.0) (struct :`Yaw` -90.0) false false))

(event `ShootBP`
  ;[1 1 1] Stop &  start shooting functions
  (`Weapon.SetCanShoot` (`self.m_weapon`) true))

(event `StopShootBP`
  ;[1 1 1] Stop &  start shooting functions
  (`Weapon.SetCanShoot` (`self.m_weapon`) false))

(event `self.AIPerception.OnTargetPerceptionUpdated`
  (params (Actor :type "Actor Object Reference") (Stimulus :type "AIStimulus Structure"))
  ;[1 1 1] Set bool to true if palyer is on sight
  (cast `/Game/BluePrints/Player/PlayerBP` Actor)
  (`BlackboardComponent.SetValueAsBool` (`AIBlueprintHelperLibrary.GetBlackboard` null) "PlayerOnSight" Stimulus_bSuccessfullySensed))

(fn `UserConstructionScript`)