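; PlayerBP is a player Blueprint with a first-person camera that sets up the player's UI and fires a test line trace.
; On BeginPlay it creates the PlayerUI widget, stores it, adds it to the viewport and makes it visible.
; Pressing E traces forward from the camera on the Camera channel with debug drawing, but nothing uses the hit result yet.
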(event `self.ReceiveBeginPlay`
  (bind _returnvalue (`|CreateWidget` "/Game/BluePrints/UI/PlayerUI.PlayerUI_C"))
  (bind _output_get (set `self.PlayerUI` _returnvalue))
  (`UserWidget.AddToViewport` _output_get 0)
  (`Widget.SetVisibility` (`self.PlayerUI`) "Visible"))

(event `Key|E`
  (params (Key :type "Key Structure"))
  (bind _firstpersoncameracomponent (`self.FirstPersonCameraComponent`))
  (bind _returnvalue (`SceneComponent.K2_GetComponentLocation` _firstpersoncameracomponent))
  (:`Pressed`
    (`KismetSystemLibrary.LineTraceSingle` :`Start` _returnvalue :`End` (+ _returnvalue (* (`SceneComponent.GetForwardVector` _firstpersoncameracomponent) 1000.0)) :`TraceChannel` "TraceTypeQuery2" :`DrawDebugType` "ForDuration")))

(fn `UserConstructionScript`)